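; BP_Torch is a torch Blueprint that can pulse its point light between minimum and maximum intensity.
; The ChangeIntensity event flip-flops a timeline between forward and reverse playback, re-entering on each finish to loop continuously.
; Timeline updates lerp the light intensity and print the curve value to screen.
; BeginPlay is empty and the only ChangeIntensity call is disconnected, so this graph never starts the pulse itself.
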(event `self.ReceiveBeginPlay`)

(event `ChangeIntensity`
  (bind _output_get (set `self.A` (not (`self.A`)) :!label _label))
  (if _output_get
    (bind (_direction _valueovertime) (`Timeline|Timeline` :!via `PlayFromStart` :!label _label_2)
      (:`Update`
        (`KismetSystemLibrary.PrintString` (`KismetStringLibrary.Conv_DoubleToString` _valueovertime))
        (`LightComponent.SetIntensity` (`self.PointLight`) (`KismetMathLibrary.Lerp` (`self.MinLightIntensity`) (`self.MaxLightIntensity`) _valueovertime)))
      (:`Finished`
        (goto _label)))
    (else
      (goto _label_2 :!via `ReverseFromEnd`))))

(fn `UserConstructionScript`)