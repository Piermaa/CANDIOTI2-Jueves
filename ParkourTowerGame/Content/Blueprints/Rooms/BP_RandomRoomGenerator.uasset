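; Room generator that spawns a sequence of random modules at preset spawn points, avoiding consecutive repeats and ending with a final room.
; Rooms spawn hidden without collision; the first two are enabled at start.
; Module-reached events from BP_EventsManager enable the room two ahead and move a fake ceiling above it.
; It also sets BP_Lava's height limit from the last spawn point and shows a progress widget when lava begins.
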(event `self.ReceiveBeginPlay`
  (bind (_returnvalue_x _returnvalue_y _returnvalue_z) (`KismetMathLibrary.BreakVector` (`self.K2_GetActorLocation`)))
  (bind _spawnpoints (`self.Spawnpoints`))
  (bind _spawnedrooms (`self.SpawnedRooms`))
  (`KismetSystemLibrary.Delay` 0.06)
  (`|ExecutionSequence`
    (:`then_0`
      (bind _returnvalue (`GameplayStatics.GetActorOfClass` "/Game/Blueprints/BP_EventsManager.BP_EventsManager_C"))
      (bind _output_get (set `self.EventsManager` _returnvalue))
      (add `/Game/Blueprints/BP_EventsManager.ModuleReached` _output_get (delegate `OnModuleReached`)))
    (:`then_1`
      (for _array_element (`self.Spawnpoints`)
        (`self.SpawnModule` _array_element))
      (`self.Enable Module` (`|GetArrayItem` _spawnedrooms))
      (`self.Enable Module` (`|GetArrayItem` _spawnedrooms 1)))
    (:`then_2`
      (add `/Game/Blueprints/BP_EventsManager.BeginLava` (`self.EventsManager`) (delegate `AddToViewPort`))
      (bind _returnvalue_2 (`GameplayStatics.GetActorOfClass` "/Game/Blueprints/BP_Lava.BP_Lava_C"))
      (set `/Game/Blueprints/BP_Lava.TopHeight` (- (+ (.z (.location (`|GetArrayItem` _spawnpoints (- (`KismetArrayLibrary.Array_Length` _spawnpoints) 1)))) _returnvalue_z) 300.0) _returnvalue_2))))

(event `AddToViewPort`
  (bind (_returnvalue_x _returnvalue_y _returnvalue_z) (`KismetMathLibrary.BreakVector` (`self.K2_GetActorLocation`)))
  (bind _spawnpoints (`self.Spawnpoints`))
  (bind _returnvalue (`|CreateWidget` "/Game/Blueprints/UI/BP_LavaProgress.BP_LavaProgress_C"))
  (`UserWidget.AddToViewport` _returnvalue 0)
  (bind (_returnvalue_x_2 _returnvalue_y_2 _returnvalue_z_2) (`KismetMathLibrary.BreakVector` (`self.K2_GetActorLocation` (stale `self.ReceiveBeginPlay` _returnvalue_2))))
  (set `/Game/Blueprints/UI/BP_LavaProgress.BaseHeight` _returnvalue_z_2 _returnvalue)
  (set `/Game/Blueprints/UI/BP_LavaProgress.TopHeight` (+ (.z (.location (`|GetArrayItem` _spawnpoints (- (`KismetArrayLibrary.Array_Length` _spawnpoints) 1)))) _returnvalue_z) _returnvalue))

(event `OnModuleReached`
  (params (ModuleIndex :type Integer))
  (bind _returnvalue (+ ModuleIndex 2))
  (bind _spawnedrooms (`self.SpawnedRooms`))
  (bind _output_location (`KismetMathLibrary.BreakTransform` (`|GetArrayItem` (`self.Spawnpoints`) _returnvalue)))
  (if (> (`KismetArrayLibrary.Array_Length` _spawnedrooms) _returnvalue)
    (`self.Enable Module` (`|GetArrayItem` _spawnedrooms _returnvalue))
    (`self.K2_SetActorLocation` (`self.FakeCeling`) (+ _output_location (0.0 0.0 1700.0)) false true)))

(fn `Enable Module`
  (params (Module :type "/Game/Blueprints/Rooms/BP_TowerRoomBase Object Reference"))
  (bind _rootcomponent (`Actor.RootComponent` Module))
  (if (not (`SceneComponent.IsVisible` _rootcomponent))
    (`SceneComponent.SetVisibility` _rootcomponent true true)
    (`self.SetActorEnableCollision` Module true)))

(fn `SpawnModule`
  (params (`Spawn Transform` :type "Transform Structure"))
  (bind _spawnpoints (`self.Spawnpoints`))
  (if (== `Spawn Transform` (`|GetArrayItem` _spawnpoints (- (`KismetArrayLibrary.Array_Length` _spawnpoints) 1)))
    (bind _returnvalue (`|SpawnActorFromClass` (`self.FinalRoom`) `Spawn Transform` "Undefined" "OverrideRootScale" null null))
    (`SceneComponent.SetVisibility` (`Actor.RootComponent` _returnvalue) false true)
    (`self.SetActorEnableCollision` _returnvalue false)
    (bind _returnvalue_2 (`KismetArrayLibrary.Array_Add` (`self.SpawnedRooms`) _returnvalue))
    (set `/Game/Blueprints/Rooms/BP_TowerRoomBase.Index` _returnvalue_2 _returnvalue)
    (set `self.LastSpawnedRoom` (`self.SelectedRoom`))
    (else
      ;[1 1 1] Genera room rd hasta generar uno distinto
      (bind _output_get (set `self.SelectedRoom` (`self.GetRandomRoom`) :!label _label))
      (if (not (== _output_get (`self.LastSpawnedRoom`)))
        (bind _returnvalue_3 (`|SpawnActorFromClass` _output_get `Spawn Transform` "Undefined" "OverrideRootScale" null null))
        (`SceneComponent.SetVisibility` (`Actor.RootComponent` _returnvalue_3) false true)
        (`self.SetActorEnableCollision` _returnvalue_3 false)
        (bind _returnvalue_4 (`KismetArrayLibrary.Array_Add` (`self.SpawnedRooms`) _returnvalue_3))
        (set `/Game/Blueprints/Rooms/BP_TowerRoomBase.Index` _returnvalue_4 _returnvalue_3)
        (set `self.LastSpawnedRoom` (`self.SelectedRoom`))
        (else
          (goto _label))))))

(fn `UserConstructionScript`)