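; BP_TowerRoomBase is a base actor for tower rooms, handling checkpoints and reactions to rising or moving lava through overlap triggers.
; Its checkpoint trigger sends damageable actors a respawn position and reports the room's Index to BP_EventsManager, found on BeginPlay.
; Lava actors, detected by interface, receive a reset position from one trigger and make the room hide and disable collision at another.
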(event `self.ReceiveBeginPlay`
  (bind _returnvalue (`GameplayStatics.GetActorOfClass` "/Game/Blueprints/BP_EventsManager.BP_EventsManager_C"))
  (set `self.EventsManager` _returnvalue))

(event `self.RoomCheckpointTrigger.OnComponentBeginOverlap`
  (params (OverlappedComponent :type "PrimitiveComponent Object Reference") (OtherActor :type "Actor Object Reference") (OtherComp :type "PrimitiveComponent Object Reference") (OtherBodyIndex :type Integer) (bFromSweep :type Boolean) (SweepResult :type "HitResult Structure (by ref)"))
  (if (`KismetSystemLibrary.DoesImplementInterface` OtherActor "/Game/Blueprints/Interfaces/BI_Damageable.BI_Damageable_C")
    (message `/Game/Blueprints/Interfaces/BI_Damageable.SetRespawnPoint` OtherActor (`SceneComponent.K2_GetComponentLocation` (`self.RoomPlayerRespawnPosition`)))
    (`/Game/Blueprints/BP_EventsManager.ModuleReached` (`self.EventsManager`) (`self.Index`))))

(event `self.ModuleDestructorTrigger.OnComponentBeginOverlap`
  (params (OverlappedComponent :type "PrimitiveComponent Object Reference") (OtherActor :type "Actor Object Reference") (OtherComp :type "PrimitiveComponent Object Reference") (OtherBodyIndex :type Integer) (bFromSweep :type Boolean) (SweepResult :type "HitResult Structure (by ref)"))
  (if (`KismetSystemLibrary.DoesImplementInterface` OtherActor "/Game/Blueprints/Interfaces/BI_Lava.BI_Lava_C")
    (`SceneComponent.SetVisibility` (`self.DefaultSceneRoot`) false true)
    (`self.SetActorEnableCollision` false)))

(event `self.LavaResetPositionTrigger.OnComponentBeginOverlap`
  (params (OverlappedComponent :type "PrimitiveComponent Object Reference") (OtherActor :type "Actor Object Reference") (OtherComp :type "PrimitiveComponent Object Reference") (OtherBodyIndex :type Integer) (bFromSweep :type Boolean) (SweepResult :type "HitResult Structure (by ref)"))
  (if (`KismetSystemLibrary.DoesImplementInterface` OtherActor "/Game/Blueprints/Interfaces/BI_Lava.BI_Lava_C")
    (message `/Game/Blueprints/Interfaces/BI_Lava.SetLavaResetPosition` OtherActor (`SceneComponent.K2_GetComponentLocation` OverlappedComponent))))

(fn `UserConstructionScript`)