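; BP_CheckPoint is a checkpoint actor that updates the player's respawn point when the player character overlaps it.
; On overlap with player character 0, it fires SetCheckPoint, which casts the game instance to BP_GameInstance and writes that instance's RespawnPoint.
; The saved point is the checkpoint's actor location plus its own RespawnPoint offset, added in world space without applying actor rotation.
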(event `self.ReceiveActorBeginOverlap`
  (params (OtherActor :type "Actor Object Reference"))
  (if (== OtherActor (`GameplayStatics.GetPlayerCharacter` 0))
    (`self.SetCheckPoint`)))

(event `SetCheckPoint`
  (bind _asbp_game_instance (cast `/Game/Blueprints/BP_GameInstance` (`GameplayStatics.GetGameInstance`)))
  (set `/Game/Blueprints/BP_GameInstance.RespawnPoint` (+ (`self.RespawnPoint`) (`self.K2_GetActorLocation`)) _asbp_game_instance))

(fn `UserConstructionScript`)