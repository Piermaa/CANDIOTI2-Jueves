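; BP_LavaLeverInteractable is an interactable lever that triggers the lava event when used.
; On interact, a timeline lerps Box1's pitch from its initial to its finish rotation, animating the pull.
; When the timeline finishes, it finds the BP_EventsManager actor in the level and calls CallBeginLava on it.
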(event `/Game/Blueprints/Interfaces/BI_Interactable.OnInteract`
  (bind _box1 (`self.Box1`))
  (bind (_relativerotation_roll _relativerotation_pitch _relativerotation_yaw) (`KismetMathLibrary.BreakRotator` (`SceneComponent.RelativeRotation` _box1)))
  (bind (_direction _newtrack_0) (`Timeline|Timeline`)
    (:`Update`
      (`SceneComponent.K2_SetRelativeRotation` _box1 (`KismetMathLibrary.MakeRotator` _relativerotation_roll (`KismetMathLibrary.Lerp` (`self.InitialRotation`) (`self.FinishRotation`) _newtrack_0) _relativerotation_yaw) false false))
    (:`Finished`
      (bind _returnvalue (`GameplayStatics.GetActorOfClass` "/Game/Blueprints/BP_EventsManager.BP_EventsManager_C"))
      (`/Game/Blueprints/BP_EventsManager.BeginLava` _returnvalue))))

(fn `UserConstructionScript`
  (`parent.UserConstructionScript`))