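; BP_Jumper is a jump-pad obstacle that launches BP_Player straight up when its Cylinder is hit.
; The hit event fires only for an exactly downward impact normal, then launches the character by LaunchPower, overriding all existing velocity.
; It plays the jumper sound at the world origin, then briefly drops and restores the Cylinder as recoil using short delays and world offsets.
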(event `self.Cylinder.OnComponentHit`
  (params (HitComponent :type "PrimitiveComponent Object Reference") (OtherActor :type "Actor Object Reference") (OtherComp :type "PrimitiveComponent Object Reference") (NormalImpulse :type "Vector Structure") (Hit :type "HitResult Structure (by ref)"))
  (bind _asbp_player (cast `/Game/ThirdPersonBP/Blueprints/BP_Player` OtherActor))
  (`/Engine/EditorBlueprintResources/StandardMacros.IsValid` _asbp_player
    (:`Is Valid`
      (if (== Hit_ImpactNormal (0.0 0.0 -1.0))
        (`Character.LaunchCharacter` _asbp_player (* (`KismetMathLibrary.Vector_Up`) (`self.LaunchPower`)) true true)
        (`GameplayStatics.PlaySoundAtLocation` "/Game/Audio/SFX/Obstacles/A_JumperSFX_Cue.A_JumperSFX_Cue" (0.0 0.0 0.0) (struct) 1.0 1.0 0.0 null null null null)
        (`KismetSystemLibrary.Delay` 0.05)
        (`SceneComponent.K2_AddWorldOffset` (`self.Cylinder`) (`KismetMathLibrary.MakeVector` 0.0 0.0 (* -1.0 (`self.LauncherRecoilDownDistance`))) false false)
        (`KismetSystemLibrary.Delay` 0.05)
        (`SceneComponent.K2_AddWorldOffset` (`self.Cylinder`) (`KismetMathLibrary.MakeVector` 0.0 0.0 (* 1.0 (`self.LauncherRecoilDownDistance`))) false false)))))

(fn `UserConstructionScript`)