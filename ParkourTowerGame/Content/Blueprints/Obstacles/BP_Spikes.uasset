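; BP_Spikes is a trap obstacle whose three spikes move when the player enters or leaves its trigger area.
; Overlap begin and end play separate up and down timelines, whose output is applied to every spike as a world Z offset on each update.
; Spike hits send BI_Damageable actors one damage and a launch opposite the trap's forward vector, scaled by KnockbackForce.
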(event `self.ReceiveBeginPlay`
  (set `self.Spikes` (`|MakeArray` (`self.Spike0`) (`self.Spike1`) (`self.Spike2`))))

(event `self.TriggerArea.OnComponentBeginOverlap`
  (params (OverlappedComponent :type "PrimitiveComponent Object Reference") (OtherActor :type "Actor Object Reference") (OtherComp :type "PrimitiveComponent Object Reference") (OtherBodyIndex :type Integer) (bFromSweep :type Boolean) (SweepResult :type "HitResult Structure (by ref)"))
  (bind _asbp_player (cast `/Game/ThirdPersonBP/Blueprints/BP_Player` OtherActor))
  (`/Engine/EditorBlueprintResources/StandardMacros.IsValid` _asbp_player
    (:`Is Valid`
      (bind (_direction _movedistance) (`Timeline|TL_SpikesUp` :!via `PlayFromStart`)
        (:`Update`
          (`self.MoveSpikes` _movedistance))))))

(event `self.TriggerArea.OnComponentEndOverlap`
  (params (OverlappedComponent :type "PrimitiveComponent Object Reference") (OtherActor :type "Actor Object Reference") (OtherComp :type "PrimitiveComponent Object Reference") (OtherBodyIndex :type Integer))
  (bind _asbp_player (cast `/Game/ThirdPersonBP/Blueprints/BP_Player` OtherActor))
  (`/Engine/EditorBlueprintResources/StandardMacros.IsValid` _asbp_player
    (:`Is Valid`
      (bind (_direction _movedistance) (`Timeline|TL_SpikesDown` :!via `PlayFromStart`)
        (:`Update`
          (`self.MoveSpikes` _movedistance))))))

(event `self.Spike0.OnComponentHit`
  (params (HitComponent :type "PrimitiveComponent Object Reference") (OtherActor :type "Actor Object Reference") (OtherComp :type "PrimitiveComponent Object Reference") (NormalImpulse :type "Vector Structure") (Hit :type "HitResult Structure (by ref)"))
  (`self.KnockCharacterBack` OtherActor))

(event `self.Spike1.OnComponentHit`
  (params (HitComponent :type "PrimitiveComponent Object Reference") (OtherActor :type "Actor Object Reference") (OtherComp :type "PrimitiveComponent Object Reference") (NormalImpulse :type "Vector Structure") (Hit :type "HitResult Structure (by ref)"))
  (`self.KnockCharacterBack` OtherActor))

(event `self.Spike2.OnComponentHit`
  (params (HitComponent :type "PrimitiveComponent Object Reference") (OtherActor :type "Actor Object Reference") (OtherComp :type "PrimitiveComponent Object Reference") (NormalImpulse :type "Vector Structure") (Hit :type "HitResult Structure (by ref)"))
  (`self.KnockCharacterBack` OtherActor))

(fn `KnockCharacterBack`
  (params (Character :type "Object Object Reference"))
  (if (`KismetSystemLibrary.DoesImplementInterface` Character "/Game/Blueprints/Interfaces/BI_Damageable.BI_Damageable_C")
    (message `/Game/Blueprints/Interfaces/BI_Damageable.TakeDamage` Character 1 (* (`self.GetActorForwardVector`) (-1.0 -1.0 -1.0)) (`self.KnockbackForce`))))

(fn `MoveSpikes`
  (params (DeltaLocation_Z :type "Float (double-precision)"))
  (for _array_element (`self.Spikes`)
    (`SceneComponent.K2_AddWorldOffset` _array_element (`KismetMathLibrary.MakeVector` 0.0 0.0 DeltaLocation_Z) false false)))

(fn `UserConstructionScript`)