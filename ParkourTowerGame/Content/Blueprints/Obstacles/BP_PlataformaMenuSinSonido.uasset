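; Moving platform obstacle, named as the soundless menu variant, that shuttles back and forth along its velocity vector.
; Tick moves it by setting its location, then snaps to the endpoint and flips velocity once travel exceeds the maximum distance.
; A player box component overlapping Bottom freezes it and plays a stop sound at world origin; the player's end overlap resumes it.
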(event `self.ReceiveBeginPlay`
  (set `self.StartLocation` (`self.K2_GetActorLocation`)))

(event `self.ReceiveTick`
  (params (DeltaSeconds :type "Float (single-precision)"))
  (if (`self.bIsFrozen`)
    _
    (elif (`self.ShouldPlatformGoBack`)
      (`self.ReversePlatformDirection`)
      (else
        (`self.MovePlatformForward` DeltaSeconds)))))

(event `self.Bottom.OnComponentBeginOverlap`
  (params (OverlappedComponent :type "PrimitiveComponent Object Reference") (OtherActor :type "Actor Object Reference") (OtherComp :type "PrimitiveComponent Object Reference") (OtherBodyIndex :type Integer) (bFromSweep :type Boolean) (SweepResult :type "HitResult Structure (by ref)"))
  (cast `/Game/ThirdPersonBP/Blueprints/BP_Player` OtherActor)
  (bind _asbox_collision (cast `BoxComponent` OtherComp))
  (`/Engine/EditorBlueprintResources/StandardMacros.IsValid` _asbox_collision
    (:`Is Valid`
      (set `self.bIsFrozen` true)
      (`GameplayStatics.PlaySoundAtLocation` "/Game/Audio/SFX/Obstacles/A_PlatformStop_SFX_Cue.A_PlatformStop_SFX_Cue" (0.0 0.0 0.0) (struct) 1.0 1.0 0.0 null null null null))
    (:`Is Not Valid`
      (set `self.bIsFrozen` false))))

(event `self.Bottom.OnComponentEndOverlap`
  (params (OverlappedComponent :type "PrimitiveComponent Object Reference") (OtherActor :type "Actor Object Reference") (OtherComp :type "PrimitiveComponent Object Reference") (OtherBodyIndex :type Integer))
  (bind _asbp_player (cast `/Game/ThirdPersonBP/Blueprints/BP_Player` OtherActor))
  (`/Engine/EditorBlueprintResources/StandardMacros.IsValid` _asbp_player
    (:`Is Valid`
      (set `self.bIsFrozen` false))))

(fn `GetDistanceTraveled`
  (returns (DistanceTraveled :type "Float (double-precision)"))
  (return (`KismetMathLibrary.Vector_Distance` (`self.StartLocation`) (`self.K2_GetActorLocation`))))

(fn `MovePlatformForward`
  (params (DeltaTime :type "Float (single-precision)"))
  (`self.K2_SetActorLocation` (+ (* DeltaTime (`self.MoveVelocity`)) (`self.K2_GetActorLocation`))))

(fn `ReversePlatformDirection`
  (locals (MoveDirection :type "Vector Structure"))
  (bind _output_get (set `local.MoveDirection` (`KismetMathLibrary.Normal` (`self.MoveVelocity`))))
  (bind _output_get_2 (set `self.StartLocation` (+ (* _output_get (`self.MaxMoveDistance`)) (`self.StartLocation`))))
  (`self.K2_SetActorLocation` _output_get_2)
  (set `self.MoveVelocity` (* (`self.MoveVelocity`) (-1.0 -1.0 -1.0))))

(fn `ShouldPlatformGoBack`
  (returns (ReverseMovement :type Boolean))
  (return (> (`self.GetDistanceTraveled`) (`self.MaxMoveDistance`))))

(fn `UserConstructionScript`)