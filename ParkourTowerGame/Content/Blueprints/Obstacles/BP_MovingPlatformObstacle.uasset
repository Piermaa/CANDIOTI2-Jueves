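; Moving platform obstacle that shuttles back and forth along its velocity vector over a set maximum distance.
; Tick moves it without sweeping; at each apex it snaps to the endpoint, reverses velocity and freezes for a delay before resuming.
; A Bottom overlap with the player's box component also freezes it until the overlap ends.
; Movement audio plays while traveling, with a stop sound on player blocks and optionally at each apex.
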(event `self.ReceiveBeginPlay`
  (set `self.StartLocation` (`self.K2_GetActorLocation`))
  (`AudioComponent.Play` (`self.AudioCurveSource`) 0.0))

(event `self.ReceiveTick`
  (params (DeltaSeconds :type "Float (single-precision)"))
  (if (`self.bIsFrozen`)
    _
    (elif (`self.ShouldPlatformGoBack`)
      (`self.ReversePlatformDirection`)
      (`|ExecutionSequence`
        (:`then_0`
          (`KismetSystemLibrary.Delay` (`self.DelayDuration`))
          (set `self.bIsFrozen` false)
          (`AudioComponent.Play` (`self.AudioCurveSource`) 0.0))
        (:`then_1`
          (if (`self.StopSFXOnApex`)
            (`self.PlayStopSFX`))))
      (else
        (`self.MovePlatformForward` DeltaSeconds)))))

(event `self.Bottom.OnComponentBeginOverlap`
  (params (OverlappedComponent :type "PrimitiveComponent Object Reference") (OtherActor :type "Actor Object Reference") (OtherComp :type "PrimitiveComponent Object Reference") (OtherBodyIndex :type Integer) (bFromSweep :type Boolean) (SweepResult :type "HitResult Structure (by ref)"))
  (cast `/Game/ThirdPersonBP/Blueprints/BP_Player` OtherActor)
  (bind _asbox_collision (cast `BoxComponent` OtherComp))
  (`/Engine/EditorBlueprintResources/StandardMacros.IsValid` _asbox_collision
    (:`Is Valid`
      (set `self.bIsFrozen` true)
      (`self.PlayStopSFX`))
    (:`Is Not Valid`
      (set `self.bIsFrozen` false))))

(event `self.Bottom.OnComponentEndOverlap`
  (params (OverlappedComponent :type "PrimitiveComponent Object Reference") (OtherActor :type "Actor Object Reference") (OtherComp :type "PrimitiveComponent Object Reference") (OtherBodyIndex :type Integer))
  (bind _asbp_player (cast `/Game/ThirdPersonBP/Blueprints/BP_Player` OtherActor))
  (`/Engine/EditorBlueprintResources/StandardMacros.IsValid` _asbp_player
    (:`Is Valid`
      (set `self.bIsFrozen` false)
      (`AudioComponent.Play` (`self.AudioCurveSource`) 0.0))))

(fn `GetDistanceTraveled`
  (returns (DistanceTraveled :type "Float (double-precision)"))
  (return (`KismetMathLibrary.Vector_Distance` (`self.StartLocation`) (`self.K2_GetActorLocation`))))

(fn `MovePlatformForward`
  (params (DeltaTime :type "Float (single-precision)"))
  (`self.K2_SetActorLocation` (+ (* DeltaTime (`self.MoveVelocity`)) (`self.K2_GetActorLocation`))))

(fn `PlayStopSFX`
  (`AudioComponent.Play` (`self.AudioCurveSourceStopSFX`) 0.0)
  (`AudioComponent.Stop` (`self.AudioCurveSource`)))

(fn `ReversePlatformDirection`
  (locals (MoveDirection :type "Vector Structure"))
  (bind _output_get (set `local.MoveDirection` (`KismetMathLibrary.Normal` (`self.MoveVelocity`))))
  (bind _output_get_2 (set `self.StartLocation` (+ (* _output_get (`self.MaxMoveDistance`)) (`self.StartLocation`))))
  (`self.K2_SetActorLocation` _output_get_2)
  (set `self.MoveVelocity` (* (`self.MoveVelocity`) (-1.0 -1.0 -1.0)))
  (set `self.bIsFrozen` true))

(fn `ShouldPlatformGoBack`
  (returns (ReverseMovement :type Boolean))
  (return (> (`self.GetDistanceTraveled`) (`self.MaxMoveDistance`))))

(fn `UserConstructionScript`)