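; Spawner actor that places one random pickupable in the level when play begins.
; On BeginPlay it picks a uniformly random class from the PickupablesToBeSpawned array and spawns it at the generator's own transform.
; It spawns only that once and does not destroy itself afterwards; the construction script is empty.
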(event `self.ReceiveBeginPlay`
  (bind _pickupablestobespawned (`self.PickupablesToBeSpawned`))
  (bind _result (`/Engine/EditorBlueprintResources/StandardMacros.DecrementInt` (`KismetArrayLibrary.Array_Length` _pickupablestobespawned))
    (:`  `
      (`|SpawnActorFromClass` (`|GetArrayItem` _pickupablestobespawned (`KismetMathLibrary.RandomIntegerInRange` 0 _result)) (`self.GetTransform` self) "Undefined" "OverrideRootScale" null null))))

(fn `UserConstructionScript`)