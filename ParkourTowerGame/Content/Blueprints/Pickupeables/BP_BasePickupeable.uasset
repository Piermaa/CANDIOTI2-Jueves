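; Base pickup actor that the player collects by touching it, with an empty Pickup function as the apparent hook for child classes.
; On BeginPlay, a Timeline animates its height between points just above and below the spawn position.
; When the player pawn overlaps the Box, OnPickup calls Pickup and the actor destroys itself.
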(event `self.ReceiveBeginPlay`
  (bind (_returnvalue_x _returnvalue_y) (`KismetMathLibrary.BreakVector` (`self.K2_GetActorLocation`)))
  (bind (_returnvalue_x_2 _returnvalue_y_2 _returnvalue_z) (`KismetMathLibrary.BreakVector` (`self.K2_GetActorLocation`)))
  (set `self.LowZ` (+ _returnvalue_z -20.0))
  (set `self.TopZ` (+ _returnvalue_z 20.0))
  (bind (_direction _newtrack_0) (`Timeline|Timeline`)
    (:`Update`
      (`self.K2_SetActorLocation` (`KismetMathLibrary.MakeVector` _returnvalue_x _returnvalue_y (`KismetMathLibrary.Lerp` (`self.TopZ`) (`self.LowZ`) _newtrack_0))))))

(event `OnPickup`
  (`self.Pickup`))

(event `self.Box.OnComponentBeginOverlap`
  (params (OverlappedComponent :type "PrimitiveComponent Object Reference") (OtherActor :type "Actor Object Reference") (OtherComp :type "PrimitiveComponent Object Reference") (OtherBodyIndex :type Integer) (bFromSweep :type Boolean) (SweepResult :type "HitResult Structure (by ref)"))
  (if (== OtherActor (`GameplayStatics.GetPlayerPawn` 0))
    (`self.OnPickup`)
    (`self.K2_DestroyActor`)))

(fn `Pickup`)

(fn `UserConstructionScript`)