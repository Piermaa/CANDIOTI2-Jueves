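; BP_Lava is a rising lava hazard that damages and launches upward any damageable actor overlapping its box.
; A looping fixed-interval timer sweeps it upward along Z at MoveSpeed, pausing while a StopTime countdown runs.
; On BeginPlay it finds BP_EventsManager and binds to its events, which can pause the rise for given seconds or teleport the lava to a reset height.
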(event `self.Box.OnComponentBeginOverlap`
  (params (OverlappedComponent :type "PrimitiveComponent Object Reference") (OtherActor :type "Actor Object Reference") (OtherComp :type "PrimitiveComponent Object Reference") (OtherBodyIndex :type Integer) (bFromSweep :type Boolean) (SweepResult :type "HitResult Structure (by ref)"))
  ;[1 1 1] Acá iría la lógica de dañar al player o reiniciar el nivel
  (if (`KismetSystemLibrary.DoesImplementInterface` OtherActor "/Game/Blueprints/Interfaces/BI_Damageable.BI_Damageable_C")
    (message `/Game/Blueprints/Interfaces/BI_Damageable.TakeDamage` OtherActor 1 (`self.GetActorUpVector` OtherActor) (`self.Launch Force`))))

(event `BeginLavaMovement`
  ;[1 1 1] Lava Movement
  (`KismetSystemLibrary.K2_SetTimerDelegate` (delegate `Lava Update`) (`self.FixedTime`) true))

(event `Lava Update`
  (bind (_returnvalue_x _returnvalue_y _returnvalue_z) (`KismetMathLibrary.BreakVector` (`self.K2_GetActorLocation`)))
  ;[1 1 1] Lava Movement
  (if (> (`self.StopTime`) 0.0)
    (set `self.StopTime` (- (`self.StopTime`) (`self.FixedTime`)))
    (else
      (`self.K2_SetActorLocation` (`KismetMathLibrary.MakeVector` _returnvalue_x _returnvalue_y (+ _returnvalue_z (* (`self.FixedTime`) (`self.MoveSpeed`)))) true))))

(event `self.ReceiveBeginPlay`
  ;[1 1 1] Esto mueve la lava, los valores del timeline deben modificarse
  (bind _returnvalue (`GameplayStatics.GetActorOfClass` "/Game/Blueprints/BP_EventsManager.BP_EventsManager_C"))
  (bind _output_get (set `self.Events Manager` _returnvalue))
  (add `/Game/Blueprints/BP_EventsManager.StopLava` _output_get (delegate `StopLava`))
  (add `/Game/Blueprints/BP_EventsManager.ResetLavaPosition` _output_get (delegate `ResetLavaPosition`))
  (`self.BeginLavaMovement`))

(event `StopLava`
  (params (StopSeconds :type "Float (double-precision)"))
  (set `self.StopTime` StopSeconds))

(event `ResetLavaPosition`
  (params (`Lava Location Z ` :type "Float (double-precision)"))
  (bind (_returnvalue_x _returnvalue_y) (`KismetMathLibrary.BreakVector` (`self.K2_GetActorLocation`)))
  (`self.K2_SetActorLocation` (`KismetMathLibrary.MakeVector` _returnvalue_x _returnvalue_y `Lava Location Z `) false true))

(fn `UserConstructionScript`)