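; Animation notify that plays a surface-dependent footstep sound.
; When notified, it line traces on Visibility from the mesh owner's location down along the actor's inverted up vector.
; The hit's physical surface type selects a grass, wood or stone sound.
; Sounds play at the world origin rather than at the owner or hit location.
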(fn `Received_Notify`
  (params (MeshComp :type "SkeletalMeshComponent Object Reference") (Animation :type "AnimSequenceBase Object Reference") (EventReference :type "AnimNotifyEventReference Structure (by ref)"))
  (returns (ReturnValue :type Boolean))
  (bind _returnvalue (`ActorComponent.GetOwner` MeshComp))
  (bind _returnvalue_2 (`Actor.K2_GetActorLocation` _returnvalue))
  (bind (_outhit _returnvalue_3) (`KismetSystemLibrary.LineTraceSingle` _returnvalue_2 (+ _returnvalue_2 (* (`Actor.GetActorUpVector` _returnvalue) -200.0)) "TraceTypeQuery1"))
  (if _returnvalue_3
    (switch `EPhysicalSurface` (`GameplayStatics.GetSurfaceType` _outhit)
      (:`SurfaceType1`
        (`GameplayStatics.PlaySoundAtLocation` "/Game/Audio/SFX/Footsteps/Grass/A_Grass_Footsteps_SFX.A_Grass_Footsteps_SFX" (0.0 0.0 0.0) (struct) 1.0 1.0 0.0 null null null null))
      (:`SurfaceType2`
        (`GameplayStatics.PlaySoundAtLocation` "/Game/Audio/SFX/Footsteps/Wood/A_WoodFootsteps_Cue.A_WoodFootsteps_Cue" (0.0 0.0 0.0) (struct) 1.0 1.0 0.0 null null null null))
      (:`SurfaceType3`
        (`GameplayStatics.PlaySoundAtLocation` "/Game/Audio/SFX/Footsteps/Stone/A_StoneFootsteps_Cue.A_StoneFootsteps_Cue" (0.0 0.0 0.0) (struct) 1.0 1.0 0.0 null null null null)))
    (return false)))